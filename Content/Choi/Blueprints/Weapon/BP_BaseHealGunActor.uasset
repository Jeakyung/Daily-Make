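; BP_BaseHealGunActor is a weapon actor, named as the base for heal guns, that loads its stats from a data table.
; The Construction Script looks up RowName in WeaponDataTable and, when the row is found, copies its cost, damage, ammo, timing and range stats into the actor's variables.
; The event graph holds only empty events, so this Blueprint defines no firing or healing logic.
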(event `self.ReceiveTick`
  (params (DeltaSeconds :type "Float (single-precision)")))

(fn `UserConstructionScript`
  (bind _returnvalue (`|GetDataTableRow` "/Game/Choi/Data/WeaponDataTable.WeaponDataTable" (`self.rowName`))
    (:`then`
      (bind (_name _rank _image _cost _weaponbp _damage _ammo _reloadtime _firerate _magazine _shootingrange _attackarea) (break `/Game/Choi/Data/WeaponItemStructure` _returnvalue))
      (set `self.cost` _cost)
      (set `self.damage` _damage)
      (set `self.ammo` _ammo)
      (set `self.reloadTime` _reloadtime)
      (set `self.fireRate` _firerate)
      (set `self.magazine` _magazine)
      (set `self.shootingRange` _shootingrange)
      (set `self.attackArea` _attackarea))))