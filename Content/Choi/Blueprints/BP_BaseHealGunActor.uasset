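; BP_BaseHealGunActor is a base heal gun actor that drives an aiming laser; no healing logic appears in its graphs.
; Every Tick, UpdateLaser line-traces on the Visibility channel from FirePoint's world location toward an End point.
; It sets the AimmingLaser effect's "Beam End" vector parameter to the hit location, or to End when nothing is hit.
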(event `self.ReceiveTick`
  (params (DeltaSeconds :type "Float (single-precision)"))
  (`self.UpdateLaser`))

(fn `UpdateLaser`
  (bind _end (`self.end`))
  (bind _aimminglaser (`self.aimmingLaser`))
  (bind (_outhit _returnvalue) (`KismetSystemLibrary.LineTraceSingle` (`SceneComponent.K2_GetComponentLocation` (`self.firePoint`)) _end "TraceTypeQuery1"))
  (if _returnvalue
    (`FXSystemComponent.SetVectorParameter` _aimminglaser "Beam End" (`.Location` (`GameplayStatics.BreakHitResult` _outhit)))
    (else
      (`FXSystemComponent.SetVectorParameter` _aimminglaser "Beam End" _end))))

(fn `UserConstructionScript`)